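; BP_P38_Pawn is a player-controlled P-38 plane pawn with simple arcade flight.
; Each tick it moves forward along its local X axis at MovementSpeed and spins the left and right propellers through a shared PropellerRotation function.
; Pitch and Roll axis inputs, clamped and scaled by delta time and PlayerRotationSpeed, rotate the actor locally, with no yaw input.
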(event EventTick
  (params (DeltaSeconds :type Float%20%28single-precision%29))
  (Transformation|AddActorLocalOffset (Math|Vector|MakeVector (* (Variables|Speed|GetMovementSpeed) (Utilities|Time|GetWorldDeltaSeconds)) 0.0 0.0) false false)
  (CallFunction|PropellerRotation (Variables|Default|GetLeft))
  (CallFunction|PropellerRotation (Variables|Default|GetRight)))

(event Input|AxisEvents|InputAxisPitch
  (params (AxisValue :type Float%20%28single-precision%29))
  (Transformation|AddActorLocalRotation (Math|Rotator|MakeRotator 0.0 (* (Math|Float|Clamp(Float) AxisValue -1.0) (Utilities|Time|GetWorldDeltaSeconds) (Variables|Default|GetPlayerRotationSpeed)) 0.0) false false))

(event Input|AxisEvents|InputAxisRoll
  (params (AxisValue :type Float%20%28single-precision%29))
  (Transformation|AddActorLocalRotation (Math|Rotator|MakeRotator (* (Math|Float|Clamp(Float) AxisValue -1.0) (Utilities|Time|GetWorldDeltaSeconds) (Variables|Default|GetPlayerRotationSpeed)) 0.0 0.0) false false))

(fn ConstructionScript)

(fn PropellerRotation
  (params (WhichPropeller :type Scene%20Component%20Object%20Reference))
  (Transformation|AddRelativeRotation WhichPropeller (Math|Rotator|MakeRotator (* (Variables|Default|GetPropellerRotationSpeed) (Utilities|Time|GetWorldDeltaSeconds)) 0.0 0.0) false false))